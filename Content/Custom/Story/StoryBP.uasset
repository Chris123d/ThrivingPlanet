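; StoryBP is a Blueprint that shows two timed story cards, each with a header and text, after play begins.
; BeginPlay clears all widgets, then a Sequence starts two independent delays that each create a hidden StoryHUD widget and assign its copy.
; RemoveStoryWidget handles the whole presentation despite its name: it fades in header then body, reverses both fades and removes the widget.
; Both cards share one StoryUI reference, so their timing depends on the delay values.
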(event EventBeginPlay
  (bind _storyui (Variables|Default|GetStoryUI))
  (bind _storyui_2 (Variables|Default|GetStoryUI))
  (Viewport|RemoveAllWidgets)
  ;[1 1 1] Story UI
  (Utilities|FlowControl|Sequence
    (:then_0
      (Utilities|FlowControl|Delay (Variables|Default|GetDelay%201%20))
      (Utilities|AddStoryWidget)
      (Variables|/Game/Custom/HUD/StoryHUD.StoryHUD_C|SetStoryHeader _storyui (Variables|Default|GetStory%20Header%201))
      (Variables|/Game/Custom/HUD/StoryHUD.StoryHUD_C|SetStoryText _storyui (Variables|Default|GetStory%20Text%201))
      (Utilities|RemoveStoryWidget))
    (:then_1
      (Utilities|FlowControl|Delay (Variables|Default|GetDelay%202))
      (Utilities|AddStoryWidget)
      (Variables|/Game/Custom/HUD/StoryHUD.StoryHUD_C|SetStoryHeader _storyui_2 (Variables|Default|GetStory%20Header%202))
      (Variables|/Game/Custom/HUD/StoryHUD.StoryHUD_C|SetStoryText _storyui_2 (Variables|Default|GetStory%20Text%202))
      (Utilities|RemoveStoryWidget))))

(fn ConstructionScript)