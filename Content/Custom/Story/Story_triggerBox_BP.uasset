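; Trigger box that shows two story messages on screen the first time something overlaps it.
; On overlap it clears all widgets, then a Sequence starts two independently delayed branches, each creating a StoryHUD widget with its own header and text.
; RemoveStoryWidget fades in the header and then the body on timed delays, plays both fades in reverse, and removes the widget.
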(event OnComponentBeginOverlap(Box)
  (params (OverlappedComponent :type Primitive%20Component%20Object%20Reference) (OtherActor :type Actor%20Object%20Reference) (OtherComp :type Primitive%20Component%20Object%20Reference) (OtherBodyIndex :type Integer) (bFromSweep :type Boolean) (SweepResult :type Hit%20Result%20Structure%20%28by%20ref%29))
  (bind _storyui (Variables|Default|GetStoryUI))
  (bind _storyui_2 (Variables|Default|GetStoryUI))
  (Utilities|FlowControl|DoOnce false
    (:Completed
      (Viewport|RemoveAllWidgets)
      ;[1 1 1] Story UI
      (Utilities|FlowControl|Sequence
        (:then_0
          (Utilities|FlowControl|Delay (Variables|Default|GetDelay%201%20))
          (Utilities|AddStoryWidget)
          (Variables|/Game/Custom/HUD/StoryHUD.StoryHUD_C|SetStoryHeader _storyui (Variables|Default|GetStory%20Header%201))
          (Variables|/Game/Custom/HUD/StoryHUD.StoryHUD_C|SetStoryText _storyui (Variables|Default|GetStory%20Text%201))
          (Utilities|RemoveStoryWidget))
        (:then_1
          (Utilities|FlowControl|Delay (Variables|Default|GetDelay%202))
          (Utilities|AddStoryWidget)
          (Variables|/Game/Custom/HUD/StoryHUD.StoryHUD_C|SetStoryHeader _storyui_2 (Variables|Default|GetStory%20Header%202))
          (Variables|/Game/Custom/HUD/StoryHUD.StoryHUD_C|SetStoryText _storyui_2 (Variables|Default|GetStory%20Text%202))
          (Utilities|RemoveStoryWidget))))))

(fn ConstructionScript)