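; Story Blueprint for the ocean scene that shows a timed intro about the Great Pacific Garbage Patch and a key prompt to return to the space station.
; On BeginPlay it clears existing widgets, waits briefly, then creates a StoryHUD with hidden header and body and sets their text.
; RemoveStoryWidget runs the whole presentation, fading in header then body with delays, reversing both fades and removing the widget.
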(event EventBeginPlay
  (bind _storyui (Variables|Default|GetStoryUI))
  (Viewport|RemoveAllWidgets)
  ;[1 1 1] Story UI
  (Utilities|FlowControl|Sequence
    (:then_0
      (Utilities|FlowControl|Delay 5.0)
      (Utilities|AddStoryWidget)
      (Variables|/Game/Custom/HUD/StoryHUD.StoryHUD_C|SetStoryHeader _storyui "This is the Great Pacific Garbage Patch.")
      (Variables|/Game/Custom/HUD/StoryHUD.StoryHUD_C|SetStoryText _storyui "Press \"r\" to return to the space station.")
      (Utilities|RemoveStoryWidget))))

(fn ConstructionScript)