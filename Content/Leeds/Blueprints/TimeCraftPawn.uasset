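; Player pawn for the TimeCraft, a flyable ship for exploring Leeds country-indicator diagrams.
; Keys jump between viewpoints by moving the ship mesh, swap to the third-person character, scale speed, toggle widgets and browse countries, setting NextJump.
; Tractor beam overlaps replace captured diagrams with a brief spinning copy and a small DataLibrary copy, plotted by weighted social-foundation and biophysical scores.
; Tick's interior scan and landing-pad spawn traces are disconnected.
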(event OnComponentBeginOverlap(TractorBeam)
  (params (OverlappedComponent :type Primitive%20Component%20Object%20Reference) (OtherActor :type Actor%20Object%20Reference) (OtherComp :type Primitive%20Component%20Object%20Reference) (OtherBodyIndex :type Integer) (bFromSweep :type Boolean) (SweepResult :type Hit%20Result%20Structure%20%28by%20ref%29))
  ;[1 0 0] Tractor Beam / Picks up data targets & positions on board
  (bind _asbp_leeds_uk_diagram (Utilities|Casting|CastToBP_LeedsUK_Diagram OtherActor))
  (Development|PrintString (Utilities|String|EnumtoString (Variables|/Game/Leeds/Blueprints/BP_LeedsUK_Diagram.BP_LeedsUK_Diagram_C|GetCountryName _asbp_leeds_uk_diagram)) true true "(R=1.000000,G=1.000000,B=0.000000,A=1.000000)" 6.0)
  (Variables|Default|SetCapturedCountry (Variables|/Game/Leeds/Blueprints/BP_LeedsUK_Diagram.BP_LeedsUK_Diagram_C|GetCountryName _asbp_leeds_uk_diagram))
  (Actor|DestroyActor OtherActor)
  (bind _returnvalue (Game|SpawnActorfromClass "/Game/Leeds/Blueprints/BP_LeedsUK_Diagram.BP_LeedsUK_Diagram_C" (Math|Transform|MakeTransform "-85.000000,905.000000,225.000000" "0,90.000000, 0" "2.000000,2.000000,2.000000") "Undefined" 0 true (Variables|Default|GetCapturedCountry) 0))
  (bind _returnvalue_2 (AddComponent|AddRotatingMovementComponent _returnvalue))
  (Variables|/Script/Engine.RotatingMovementComponent|SetRotationRate _returnvalue_2 "0,100.000000, 0")
  (Actor|SetLifeSpan _returnvalue 5.0)
  (Transformation|AttachComponentToComponent _returnvalue (Variables|Default|GetTimeCraft_Merged) "None" "KeepRelative" "KeepRelative" "KeepRelative" true)
  (bind _returnvalue_3 (Game|SpawnActorfromClass "/Game/Leeds/Blueprints/BP_LeedsUK_Diagram.BP_LeedsUK_Diagram_C" (Math|Transform|MakeTransform (Math|Vector|MakeVector 0.0 -2e+02 0.0) "0.000000,90.000000,0.000000" "0.250000,0.250000,0.250000") "Undefined" 0 true (Variables|Default|GetCapturedCountry) 0))
  (Transformation|AttachComponentToComponent _returnvalue_3 (Variables|Default|GetDataLibrary) "None" "KeepRelative" "KeepRelative" "KeepWorld" true)
  (bind (_social_foundation_score _biophysical_score) (CallFunction|CalculateBoardPosition _returnvalue_3))
  (Transformation|AddActorLocalOffset _returnvalue_3 (Math|Vector|MakeVector 0.0 _social_foundation_score _biophysical_score) false false))

(event Custom|ToggleTimeOfDay
  ;[0 1 0.08171] Cesium
  ;;[0 0.3037 1] Toggle Time of Day Widget
  (bind _timeofdayref (Variables|Default|GetTimeOfDayRef)
    (:then
      (Default|Teardown _timeofdayref)
      (Variables|Default|SetTimeOfDayRef 0))
    (:else
      (bind _returnvalue (UserInterface|CreateWidget "/CesiumForUnreal/WBP_TimeOfDay.WBP_TimeOfDay_C" (Game|GetPlayerController 0)))
      (UserInterface|Viewport|AddtoViewport _returnvalue 0)
      (Variables|Default|SetTimeOfDayRef _returnvalue))))

(event EventBeginPlay
  ;[0 0 0] Begin Play - Set starting position inside of TimeCraft
  (Transformation|SetRelativeLocation (Variables|Default|GetTimeCraft_Merged) (Variables|TimeCraft|POVs|GetDataBrowser) false false)
  (Pawn|SetControlRotation (Pawn|GetController) (Math|Rotator|MakeRotator 0.0 -5.0 0.0)))

(event EventTick
  (params (DeltaSeconds :type Float%20%28single-precision%29)))

(event Input|MouseEvents|MouseWheelUp
  (params (Key :type Key%20Structure :default "None"))
  (bind _movementcomponent (Variables|Default|GetMovementComponent))
  ;[0 1 0.08171] Cesium
  ;;[0 0.3037 1] Scroll to change movement speed
  (:Pressed
    (bind _asfloating_pawn_movement (Utilities|Casting|CastToFloatingPawnMovement _movementcomponent))
    (Variables|/Script/Engine.FloatingPawnMovement|SetMaxSpeed _asfloating_pawn_movement (* (Class|MovementComponent|GetMaxSpeed _movementcomponent) (Variables|Default|GetIncrement)))))

(event Input|MouseEvents|MouseWheelDown
  (params (Key :type Key%20Structure :default "None"))
  (bind _movementcomponent (Variables|Default|GetMovementComponent))
  ;[0 1 0.08171] Cesium
  ;;[0 0.3037 1] Scroll to change movement speed
  (:Pressed
    (bind _asfloating_pawn_movement (Utilities|Casting|CastToFloatingPawnMovement _movementcomponent))
    (Variables|/Script/Engine.FloatingPawnMovement|SetMaxSpeed _asfloating_pawn_movement (/ (Class|MovementComponent|GetMaxSpeed _movementcomponent) (Variables|Default|GetDecrement)))))

(event Input|KeyboardEvents|5
  (params (Key :type Key%20Structure :default "None"))
  ;[0 0 0] Change Camera Location on Time Craft
  (:Pressed
    (Transformation|SetRelativeLocation (Variables|Default|GetTimeCraft_Merged) (Variables|TimeCraft|POVs|GetDataBrowser) false false)
    (Pawn|SetControlRotation (Pawn|GetController) (Math|Rotator|MakeRotator 0.0 -5.0 0.0))))

(event Input|KeyboardEvents|Comma
  (params (Key :type Key%20Structure :default "None"))
  ;[1 0 0] Browse Data / Set Next Jump Coordinates
  (:Pressed
    (bind _result (Math|Integer|DecrementInt (Variables|Default|GetCountryCounter))
      (:%20%20
        (bind _output_get (Variables|Default|SetCountryCounter _result))
        (Utilities|IsValid (Variables|Default|GetData)
          (:Is%20Valid
            (Actor|DestroyActor (Variables|Default|GetData)))
          (:Is%20Not%20Valid
            _))
        (Variables|Default|SetNextJump (Utilities|Enum|ByteToEnumECountries (Math|Conversions|ToByte(Integer) _output_get)))
        (bind _returnvalue (Game|SpawnActorfromClass "/Game/Leeds/Blueprints/BP_LeedsUK_Diagram.BP_LeedsUK_Diagram_C" (Math|Transform|MakeTransform "-85.000000,905.000000,225.000000" "0,90.000000, 0" "5.000000,5.000000,5.000000") "Undefined" 0 true (Utilities|Enum|ByteToEnumECountries (Math|Conversions|ToByte(Integer) _output_get)) 0))
        (bind _output_get_2 (Variables|Default|SetData _returnvalue))
        (Transformation|AttachComponentToComponent _output_get_2 (Variables|Default|GetTimeCraft_Merged) "None" "KeepRelative" "KeepRelative" "KeepRelative" true)
        (Actor|SetLifeSpan (Variables|Default|GetData) 1e+01)))))

(event Input|KeyboardEvents|8
  (params (Key :type Key%20Structure :default "None"))
  ;[0 0 0] Switch Pawns from Ship to Third Person
  (:Pressed
    (Utilities|FlowControl|FlipFlop
      (:A
        (bind _returnvalue (Actor|GetActorOfClass "/Game/CesiumSamples/Maps/03/ThirdPersonController/ThirdPersonCharacter.ThirdPersonCharacter_C"))
        (Pawn|Possess (Game|GetPlayerController 0) _returnvalue))
      (:B
        (Pawn|Possess (Game|GetPlayerController 0) self)))))

(event Input|KeyboardEvents|6
  (params (Key :type Key%20Structure :default "None"))
  ;[0 0 0] Change Camera Location on Time Craft
  (:Pressed
    (Transformation|SetRelativeLocation (Variables|Default|GetTimeCraft_Merged) (Variables|TimeCraft|POVs|GetOutsideShip) false false)
    (Pawn|SetControlRotation (Pawn|GetController) (Math|Rotator|MakeRotator 0.0 -5.0 0.0))))

(event Input|KeyboardEvents|7
  (params (Key :type Key%20Structure :default "None"))
  ;[0 0 0] Change Camera Location on Time Craft
  (:Pressed
    (Transformation|SetRelativeLocation (Variables|Default|GetTimeCraft_Merged) (Variables|TimeCraft|POVs|GetAboveShip) false false)
    (Pawn|SetControlRotation (Pawn|GetController) (Math|Rotator|MakeRotator 0.0 0.0 -1.8e+02))))

(event Input|KeyboardEvents|P
  (params (Key :type Key%20Structure :default "None"))
  ;[0 1 0.08171] Cesium
  ;;[0 0.3037 1] Toggle Profiling Widget
  (:Pressed
    (bind _profilingref (Variables|Default|GetProfilingRef)
      (:then
        (Default|Teardown _profilingref)
        (Variables|Default|SetProfilingRef 0))
      (:else
        (bind _returnvalue (UserInterface|CreateWidget "/CesiumForUnreal/WBP_Profiling.WBP_Profiling_C" (Game|GetPlayerController 0)))
        (UserInterface|Viewport|AddtoViewport _returnvalue 0)
        (Variables|Default|SetProfilingRef _returnvalue)))))

(event Input|KeyboardEvents|1
  (params (Key :type Key%20Structure :default "None"))
  ;[0 0 0] Change Camera Location on Time Craft
  (:Pressed
    (Transformation|SetRelativeLocation (Variables|Default|GetTimeCraft_Merged) (Variables|TimeCraft|POVs|GetFrontOfShip) false false)
    (Pawn|SetControlRotation (Pawn|GetController) (Math|Rotator|MakeRotator 0.0 0.0 0.0))))

(event Input|KeyboardEvents|T
  (params (Key :type Key%20Structure :default "None"))
  ;[0 1 0.08171] Cesium
  ;;[0 0.3037 1] Toggle Time of Day Widget
  (:Pressed
    (CallFunction|ToggleTimeOfDay)))

(event Input|KeyboardEvents|2
  (params (Key :type Key%20Structure :default "None"))
  ;[0 0 0] Change Camera Location on Time Craft
  (:Pressed
    (Transformation|SetRelativeLocation (Variables|Default|GetTimeCraft_Merged) (Variables|TimeCraft|POVs|GetCentral) false false)
    (Pawn|SetControlRotation (Pawn|GetController) (Math|Rotator|MakeRotator 0.0 -9e+01 0.0))))

(event Input|KeyboardEvents|3
  (params (Key :type Key%20Structure :default "None"))
  ;[0 0 0] Change Camera Location on Time Craft
  (:Pressed
    (Transformation|SetRelativeLocation (Variables|Default|GetTimeCraft_Merged) (Variables|TimeCraft|POVs|GetDataInspector) false false)
    (Pawn|SetControlRotation (Pawn|GetController) (Math|Rotator|MakeRotator 0.0 9.0 85.0))))

(event Input|KeyboardEvents|4
  (params (Key :type Key%20Structure :default "None"))
  ;[0 0 0] Change Camera Location on Time Craft
  (:Pressed
    (Transformation|SetRelativeLocation (Variables|Default|GetTimeCraft_Merged) (Variables|TimeCraft|POVs|GetCrew_1) false false)
    (Pawn|SetControlRotation (Pawn|GetController) (Math|Rotator|MakeRotator 0.0 0.0 -6e+01))))

(event Input|KeyboardEvents|Period
  (params (Key :type Key%20Structure :default "None"))
  ;[1 0 0] Browse Data / Set Next Jump Coordinates
  (:Pressed
    (bind _result (Math|Integer|IncrementInt (Variables|Default|GetCountryCounter))
      (:%20%20
        (bind _output_get (Variables|Default|SetCountryCounter _result))
        (Utilities|IsValid (Variables|Default|GetData)
          (:Is%20Valid
            (Actor|DestroyActor (Variables|Default|GetData)))
          (:Is%20Not%20Valid
            _))
        (Variables|Default|SetNextJump (Utilities|Enum|ByteToEnumECountries (Math|Conversions|ToByte(Integer) _output_get)))
        (bind _returnvalue (Game|SpawnActorfromClass "/Game/Leeds/Blueprints/BP_LeedsUK_Diagram.BP_LeedsUK_Diagram_C" (Math|Transform|MakeTransform "-85.000000,905.000000,225.000000" "0,90.000000, 0" "5.000000,5.000000,5.000000") "Undefined" 0 true (Utilities|Enum|ByteToEnumECountries (Math|Conversions|ToByte(Integer) _output_get)) 0))
        (bind _output_get_2 (Variables|Default|SetData _returnvalue))
        (Transformation|AttachComponentToComponent _output_get_2 (Variables|Default|GetTimeCraft_Merged) "None" "KeepRelative" "KeepRelative" "KeepRelative" true)
        (Actor|SetLifeSpan (Variables|Default|GetData) 1e+01)))))

(fn ConstructionScript)

(fn CalculateBoardPosition
  (params (Country :type BP%20Leeds%20UK%20Diagram%20Object%20Reference))
  (bind (_countryout _biophysical_score) (Utilities|CalculateBiophysicalScore Country))
  (bind _social_foundation_score (Utilities|CalculateSocialFoundationScore _countryout))
  (return _social_foundation_score _biophysical_score))