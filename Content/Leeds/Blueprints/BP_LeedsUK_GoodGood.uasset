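; Leeds UK indicator chart actor that draws social and biophysical data as radial segments, resembling a Doughnut Economics diagram.
; The construction script reads two DataTable rows by CountryName and scales them, splitting biophysical values above 1.0 into capped under and overshoot radii.
; Dynamic material instances receive each value as a Radius parameter.
; SetCountryName selects table-driven radii and the country label, otherwise manually set variables drive the radii.
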(event EventBeginPlay)

(event Collision|EventActorBeginOverlap
  (params (OtherActor :type Actor%20Object%20Reference)))

(event EventTick
  (params (DeltaSeconds :type Float%20%28single-precision%29)))

(fn ConstructionScript
  (Utilities|FlowControl|Sequence
    (:then_0
      (bind _returnvalue (Utilities|GetDataTableRow "/Game/Leeds/Data/DT_SocialIndicators_LeedsUK.DT_SocialIndicators_LeedsUK" (Utilities|String|StringToName (Utilities|String|EnumtoString (Variables|LeedsUKData|GetCountryName))))
        (:then
          (Variables|LeedsUKData|Social|SetLife%20Satisfaction%20%28scaled%29 (* (/ (.lifesatisfaction _returnvalue) 1.36) 16.1))
          (Variables|LeedsUKData|Social|SetHealthy%20Life%20Expectancy%20%28scaled%29 (* (/ (.healthylifeexpect _returnvalue) 1.37) 16.1))
          (Variables|LeedsUKData|Social|SetNutrition%20%28scaled%29 (* (/ (.nutrition _returnvalue) 2.09) 16.1))
          (Variables|LeedsUKData|Social|SetSanitation%20%28scaled%29 (* (/ (.sanitation _returnvalue) 1.06) 16.1))
          (Variables|LeedsUKData|Social|SetIncome%20%28scaled%29 (* (/ (.income _returnvalue) 1.07) 16.1))
          (Variables|LeedsUKData|Social|SetAccess%20to%20Energy%20%28scaled%29 (* (/ (.accesstoenergy _returnvalue) 1.06) 16.1))
          (Variables|LeedsUKData|Social|SetEducation%20%28scaled%29 (* (/ (.education _returnvalue) 1.49) 16.1))
          (Variables|LeedsUKData|Social|SetSocial%20Support%20%28scaled%29 (* (/ (.socialsupport _returnvalue) 1.13) 16.1))
          (Variables|LeedsUKData|Social|SetDemocratic%20Quality%20%28scaled%29 (* (/ (.democraticquality _returnvalue) 1.13) 16.1))
          (Variables|LeedsUKData|Social|SetEquality%20%28scaled%29 (* (/ (.equality _returnvalue) 1.13) 16.1))
          (Variables|LeedsUKData|Social|SetEmployment%20%28scaled%29 (* (/ (.employment _returnvalue) 1.13) 16.1)))))
    (:then_1
      (bind _returnvalue_2 (Utilities|GetDataTableRow "/Game/Leeds/Data/DT_BiophysicalIndicators_LeedsUK.DT_BiophysicalIndicators_LeedsUK" (Utilities|String|StringToName (Utilities|String|EnumtoString (Variables|LeedsUKData|GetCountryName))))
        (:then
          (Utilities|ScaleCO2Emissions (.co2emissions _returnvalue_2))
          (Utilities|ScalePhosphorus (.phosphorus _returnvalue_2))
          (Utilities|ScaleNitrogen (.nitrogen _returnvalue_2))
          (Utilities|ScaleBlueWater (.bluewater _returnvalue_2))
          (Utilities|ScaleLandUseChange (.ehanpp _returnvalue_2))
          (Utilities|ScaleEcologicalFootprint (.ecologicalfootprint _returnvalue_2))
          (Utilities|ScaleMaterialFootprint (.materialfootprint _returnvalue_2)))))
    (:then_2
      (if (Variables|LeedsUKData|GetSetCountryName?)
        (Rendering|Components|TextRender|SetText (Variables|Default|GetCountry) (Utilities|Text|ToText(String) (Utilities|String|EnumtoString (Variables|LeedsUKData|GetCountryName))))))
    (:then_3
      ;[1 1 1] Sanitation
      (bind _returnvalue_3 (Rendering|Material|CreateDynamicMaterialInstance (Variables|SocialFoundation|Meshes|Get1__Sanitation) 0 "/Game/Leeds/Materials/SocialFoundations/MI_Sanitation.MI_Sanitation" "None" :!class /Script/Engine.PrimitiveComponent))
      (bind _output_get (Variables|MIDynamic|SetSanitation_MI _returnvalue_3))
      (if (Variables|LeedsUKData|GetSetCountryName?)
        (Rendering|Material|SetScalarParameterValue _output_get "Radius" (Variables|LeedsUKData|Social|GetSanitation%20%28scaled%29) :!class /Script/Engine.MaterialInstanceDynamic)
        (else
          (Rendering|Material|SetScalarParameterValue _output_get "Radius" (Variables|SocialFoundation|Indicators|GetSanitation) :!class /Script/Engine.MaterialInstanceDynamic)))
      ;[1 1 1] Income
      (bind _returnvalue_4 (Rendering|Material|CreateDynamicMaterialInstance (Variables|SocialFoundation|Meshes|Get2__Income) 0 "/Game/Leeds/Materials/SocialFoundations/MI_Income.MI_Income" "None" :!class /Script/Engine.PrimitiveComponent))
      (bind _output_get_2 (Variables|MIDynamic|SetIncome_MI _returnvalue_4))
      (if (Variables|LeedsUKData|GetSetCountryName?)
        (Rendering|Material|SetScalarParameterValue _output_get_2 "Radius" (Variables|LeedsUKData|Social|GetIncome%20%28scaled%29) :!class /Script/Engine.MaterialInstanceDynamic)
        (else
          (Rendering|Material|SetScalarParameterValue _output_get_2 "Radius" (Variables|SocialFoundation|Indicators|GetIncome) :!class /Script/Engine.MaterialInstanceDynamic)))
      ;[1 1 1] Access to Energy
      (bind _returnvalue_5 (Rendering|Material|CreateDynamicMaterialInstance (Variables|SocialFoundation|Meshes|Get3__Access%20to%20Energy) 0 "/Game/Leeds/Materials/SocialFoundations/MI_Income.MI_Income" "None" :!class /Script/Engine.PrimitiveComponent))
      (bind _output_get_3 (Variables|MIDynamic|SetAccessToEnergy_MI _returnvalue_5))
      (if (Variables|LeedsUKData|GetSetCountryName?)
        (Rendering|Material|SetScalarParameterValue _output_get_3 "Radius" (Variables|LeedsUKData|Social|GetAccess%20to%20Energy%20%28scaled%29) :!class /Script/Engine.MaterialInstanceDynamic)
        (else
          (Rendering|Material|SetScalarParameterValue _output_get_3 "Radius" (Variables|SocialFoundation|Indicators|GetAcces%20to%20energy) :!class /Script/Engine.MaterialInstanceDynamic)))
      ;[1 1 1] Education
      (bind _returnvalue_6 (Rendering|Material|CreateDynamicMaterialInstance (Variables|SocialFoundation|Meshes|Get4__Education) 0 "/Game/Leeds/Materials/SocialFoundations/MI_Education.MI_Education" "None" :!class /Script/Engine.PrimitiveComponent))
      (bind _output_get_4 (Variables|MIDynamic|SetEducation_MI _returnvalue_6))
      (if (Variables|LeedsUKData|GetSetCountryName?)
        (Rendering|Material|SetScalarParameterValue _output_get_4 "Radius" (Variables|LeedsUKData|Social|GetEducation%20%28scaled%29) :!class /Script/Engine.MaterialInstanceDynamic)
        (else
          (Rendering|Material|SetScalarParameterValue _output_get_4 "Radius" (Variables|SocialFoundation|Indicators|GetEducation) :!class /Script/Engine.MaterialInstanceDynamic)))
      ;[1 1 1] Social Support
      (bind _returnvalue_7 (Rendering|Material|CreateDynamicMaterialInstance (Variables|SocialFoundation|Meshes|Get5__Social%20Support) 0 "/Game/Leeds/Materials/SocialFoundations/MI_SocialSupport.MI_SocialSupport" "None" :!class /Script/Engine.PrimitiveComponent))
      (bind _output_get_5 (Variables|MIDynamic|SetSocialSupport_MI _returnvalue_7))
      (if (Variables|LeedsUKData|GetSetCountryName?)
        (Rendering|Material|SetScalarParameterValue _output_get_5 "Radius" (Variables|LeedsUKData|Social|GetSocial%20Support%20%28scaled%29) :!class /Script/Engine.MaterialInstanceDynamic)
        (else
          (Rendering|Material|SetScalarParameterValue _output_get_5 "Radius" (Variables|SocialFoundation|Indicators|GetSocial%20Support) :!class /Script/Engine.MaterialInstanceDynamic)))
      ;[1 1 1] Democratic Quality
      (bind _returnvalue_8 (Rendering|Material|CreateDynamicMaterialInstance (Variables|SocialFoundation|Meshes|Get6__Democratic%20Quality) 0 "/Game/Leeds/Materials/SocialFoundations/MI_DemocraticQuality.MI_DemocraticQuality" "None" :!class /Script/Engine.PrimitiveComponent))
      (bind _output_get_6 (Variables|MIDynamic|SetDemocracticQuality_MI _returnvalue_8))
      (if (Variables|LeedsUKData|GetSetCountryName?)
        (Rendering|Material|SetScalarParameterValue _output_get_6 "Radius" (Variables|LeedsUKData|Social|GetDemocratic%20Quality%20%28scaled%29) :!class /Script/Engine.MaterialInstanceDynamic)
        (else
          (Rendering|Material|SetScalarParameterValue _output_get_6 "Radius" (Variables|SocialFoundation|Indicators|GetDemocratic%20Quality) :!class /Script/Engine.MaterialInstanceDynamic)))
      ;[1 1 1] Equality
      (bind _returnvalue_9 (Rendering|Material|CreateDynamicMaterialInstance (Variables|SocialFoundation|Meshes|Get7__Equality) 0 "/Game/Leeds/Materials/SocialFoundations/MI_Equality.MI_Equality" "None" :!class /Script/Engine.PrimitiveComponent))
      (bind _output_get_7 (Variables|MIDynamic|SetEquality%20MI _returnvalue_9))
      (if (Variables|LeedsUKData|GetSetCountryName?)
        (Rendering|Material|SetScalarParameterValue _output_get_7 "Radius" (Variables|LeedsUKData|Social|GetEquality%20%28scaled%29) :!class /Script/Engine.MaterialInstanceDynamic)
        (else
          (Rendering|Material|SetScalarParameterValue _output_get_7 "Radius" (Variables|SocialFoundation|Indicators|GetEquality) :!class /Script/Engine.MaterialInstanceDynamic)))
      ;[1 1 1] Employment
      (bind _returnvalue_10 (Rendering|Material|CreateDynamicMaterialInstance (Variables|SocialFoundation|Meshes|Get8__Employment) 0 "/Game/Leeds/Materials/SocialFoundations/MI_Employment.MI_Employment" "None" :!class /Script/Engine.PrimitiveComponent))
      (bind _output_get_8 (Variables|MIDynamic|SetEmployment_MI _returnvalue_10))
      (if (Variables|LeedsUKData|GetSetCountryName?)
        (Rendering|Material|SetScalarParameterValue _output_get_8 "Radius" (Variables|LeedsUKData|Social|GetEmployment%20%28scaled%29) :!class /Script/Engine.MaterialInstanceDynamic)
        (else
          (Rendering|Material|SetScalarParameterValue _output_get_8 "Radius" (Variables|SocialFoundation|Indicators|GetEmployment) :!class /Script/Engine.MaterialInstanceDynamic)))
      ;[1 1 1] Life Satisfaction
      (bind _returnvalue_11 (Rendering|Material|CreateDynamicMaterialInstance (Variables|SocialFoundation|Meshes|Get9__Life%20Satisfaction) 0 "/Game/Leeds/Materials/SocialFoundations/MI_LifeSatisfaction.MI_LifeSatisfaction" "None" :!class /Script/Engine.PrimitiveComponent))
      (bind _output_get_9 (Variables|MIDynamic|SetLifeSatisfaction_MI _returnvalue_11))
      (if (Variables|LeedsUKData|GetSetCountryName?)
        (Rendering|Material|SetScalarParameterValue _output_get_9 "Radius" (Variables|LeedsUKData|Social|GetLife%20Satisfaction%20%28scaled%29) :!class /Script/Engine.MaterialInstanceDynamic)
        (else
          (Rendering|Material|SetScalarParameterValue _output_get_9 "Radius" (Variables|SocialFoundation|Indicators|GetLife%20Satisfaction) :!class /Script/Engine.MaterialInstanceDynamic)))
      ;[1 1 1] Healthy Life Expectancy
      (bind _returnvalue_12 (Rendering|Material|CreateDynamicMaterialInstance (Variables|SocialFoundation|Meshes|Get10__Healthy%20Life%20Expectancy) 0 "/Game/Leeds/Materials/SocialFoundations/MI_HealthyLifeExpectancy.MI_HealthyLifeExpectancy" "None" :!class /Script/Engine.PrimitiveComponent))
      (bind _output_get_10 (Variables|MIDynamic|SetHealthyLifeExpectancy_MI _returnvalue_12))
      (if (Variables|LeedsUKData|GetSetCountryName?)
        (Rendering|Material|SetScalarParameterValue _output_get_10 "Radius" (Variables|LeedsUKData|Social|GetHealthy%20Life%20Expectancy%20%28scaled%29) :!class /Script/Engine.MaterialInstanceDynamic)
        (else
          (Rendering|Material|SetScalarParameterValue _output_get_10 "Radius" (Variables|SocialFoundation|Indicators|GetHealthy%20Life%20Expectancy) :!class /Script/Engine.MaterialInstanceDynamic)))
      ;[1 1 1] Nutrition
      (bind _returnvalue_13 (Rendering|Material|CreateDynamicMaterialInstance (Variables|SocialFoundation|Meshes|Get11__Nutrition) 0 "/Game/Leeds/Materials/SocialFoundations/MI_Nutrition.MI_Nutrition" "None" :!class /Script/Engine.PrimitiveComponent))
      (bind _output_get_11 (Variables|MIDynamic|SetNutrition_MI _returnvalue_13))
      (if (Variables|LeedsUKData|GetSetCountryName?)
        (Rendering|Material|SetScalarParameterValue _output_get_11 "Radius" (Variables|LeedsUKData|Social|GetNutrition%20%28scaled%29) :!class /Script/Engine.MaterialInstanceDynamic)
        (else
          (Rendering|Material|SetScalarParameterValue _output_get_11 "Radius" (Variables|SocialFoundation|Indicators|GetNutrition) :!class /Script/Engine.MaterialInstanceDynamic))))
    (:then_4
      ;[1 1 1] CO2 Emissions
      (bind _returnvalue_14 (Rendering|Material|CreateDynamicMaterialInstance (Variables|PlanetaryBoundaryMeshes|Ideal|GetCO2%20Emissions%20Under) 0 "/Game/Leeds/Materials/PlanetaryBoundariesUnder/MI_CO2EmissionsUnder.MI_CO2EmissionsUnder" "None" :!class /Script/Engine.PrimitiveComponent))
      (bind _output_get_12 (Variables|MIDynamic|SetCO2%20Emissions%20Ideal _returnvalue_14))
      (if (Variables|LeedsUKData|GetSetCountryName?)
        (Rendering|Material|SetScalarParameterValue _output_get_12 "Radius" (Variables|LeedsUKData|Biophysical|GetCO2%20Emissions%20Under%20%28scaled%29) :!class /Script/Engine.MaterialInstanceDynamic)
        (else
          (Rendering|Material|SetScalarParameterValue _output_get_12 "Radius" (Variables|PlanetaryBoundaryIndicators|Ideal|GetCO2%20Emissions%20) :!class /Script/Engine.MaterialInstanceDynamic)))
      ;[1 1 1] Phosphorus
      (bind _returnvalue_15 (Rendering|Material|CreateDynamicMaterialInstance (Variables|PlanetaryBoundaryMeshes|Ideal|GetPhosphorus%20Under) 0 "/Game/Leeds/Materials/PlanetaryBoundariesUnder/MI_PhosphorusUnder.MI_PhosphorusUnder" "None" :!class /Script/Engine.PrimitiveComponent))
      (bind _output_get_13 (Variables|MIDynamic|SetPhosphorus%20Ideal _returnvalue_15))
      (if (Variables|LeedsUKData|GetSetCountryName?)
        (Rendering|Material|SetScalarParameterValue _output_get_13 "Radius" (Variables|LeedsUKData|Biophysical|GetPhosphorus%20Under%20%28scaled%29) :!class /Script/Engine.MaterialInstanceDynamic)
        (else
          (Rendering|Material|SetScalarParameterValue _output_get_13 "Radius" (Variables|PlanetaryBoundaryIndicators|Ideal|GetPhosphorus) :!class /Script/Engine.MaterialInstanceDynamic)))
      ;[1 1 1] Nitrogen
      (bind _returnvalue_16 (Rendering|Material|CreateDynamicMaterialInstance (Variables|PlanetaryBoundaryMeshes|Ideal|GetNitrogen%20Under) 0 "/Game/Leeds/Materials/PlanetaryBoundariesUnder/MI_NitrogenUnder.MI_NitrogenUnder" "None" :!class /Script/Engine.PrimitiveComponent))
      (bind _output_get_14 (Variables|MIDynamic|SetNitrogen%20Ideal _returnvalue_16))
      (if (Variables|LeedsUKData|GetSetCountryName?)
        (Rendering|Material|SetScalarParameterValue _output_get_14 "Radius" (Variables|LeedsUKData|Biophysical|GetNitrogen%20Under%20%28scaled%29) :!class /Script/Engine.MaterialInstanceDynamic)
        (else
          (Rendering|Material|SetScalarParameterValue _output_get_14 "Radius" (Variables|PlanetaryBoundaryIndicators|Ideal|GetNitrogen) :!class /Script/Engine.MaterialInstanceDynamic)))
      ;[1 1 1] Blue Water
      (bind _returnvalue_17 (Rendering|Material|CreateDynamicMaterialInstance (Variables|PlanetaryBoundaryMeshes|Ideal|GetBlue%20Water%20Under) 0 "/Game/Leeds/Materials/PlanetaryBoundariesUnder/MI_BlueWaterUnder.MI_BlueWaterUnder" "None" :!class /Script/Engine.PrimitiveComponent))
      (bind _output_get_15 (Variables|MIDynamic|SetBlue%20Water%20Ideal _returnvalue_17))
      (if (Variables|LeedsUKData|GetSetCountryName?)
        (Rendering|Material|SetScalarParameterValue _output_get_15 "Radius" (Variables|LeedsUKData|Biophysical|GetBlue%20Water%20Under%20%28scaled%29) :!class /Script/Engine.MaterialInstanceDynamic)
        (else
          (Rendering|Material|SetScalarParameterValue _output_get_15 "Radius" (Variables|PlanetaryBoundaryIndicators|Ideal|GetBlue%20Water) :!class /Script/Engine.MaterialInstanceDynamic)))
      ;[1 1 1] Land Use Change
      (bind _returnvalue_18 (Rendering|Material|CreateDynamicMaterialInstance (Variables|PlanetaryBoundaryMeshes|Ideal|GetLand%20Use%20Change%20Under) 0 "/Game/Leeds/Materials/PlanetaryBoundariesUnder/MI_LandUseChangeUnder.MI_LandUseChangeUnder" "None" :!class /Script/Engine.PrimitiveComponent))
      (bind _output_get_16 (Variables|MIDynamic|SetLand%20Use%20Change%20Ideal _returnvalue_18))
      (if (Variables|LeedsUKData|GetSetCountryName?)
        (Rendering|Material|SetScalarParameterValue _output_get_16 "Radius" (Variables|LeedsUKData|Biophysical|GetLand%20Use%20Change%20Under%20%28scaled%29) :!class /Script/Engine.MaterialInstanceDynamic)
        (else
          (Rendering|Material|SetScalarParameterValue _output_get_16 "Radius" (Variables|PlanetaryBoundaryIndicators|Ideal|GetLand%20Use%20Change) :!class /Script/Engine.MaterialInstanceDynamic)))
      ;[1 1 1] Ecological Footprint
      (bind _returnvalue_19 (Rendering|Material|CreateDynamicMaterialInstance (Variables|PlanetaryBoundaryMeshes|Ideal|GetEcological%20Footprint%20Under) 0 "/Game/Leeds/Materials/PlanetaryBoundariesUnder/MI_EcologicalFootprintUnder.MI_EcologicalFootprintUnder" "None" :!class /Script/Engine.PrimitiveComponent))
      (bind _output_get_17 (Variables|MIDynamic|SetEcological%20Footprint%20Ideal _returnvalue_19))
      (if (Variables|LeedsUKData|GetSetCountryName?)
        (Rendering|Material|SetScalarParameterValue _output_get_17 "Radius" (Variables|LeedsUKData|Biophysical|GetEcological%20Footprint%20Under%20%28scaled%29) :!class /Script/Engine.MaterialInstanceDynamic)
        (else
          (Rendering|Material|SetScalarParameterValue _output_get_17 "Radius" (Variables|PlanetaryBoundaryIndicators|Ideal|GetEcological%20Footprint) :!class /Script/Engine.MaterialInstanceDynamic)))
      ;[1 1 1] Material Footprint
      (bind _returnvalue_20 (Rendering|Material|CreateDynamicMaterialInstance (Variables|PlanetaryBoundaryMeshes|Ideal|GetMaterial%20Footprint%20Under) 0 "/Game/Leeds/Materials/PlanetaryBoundariesUnder/MI_MaterialFootprintUnder.MI_MaterialFootprintUnder" "None" :!class /Script/Engine.PrimitiveComponent))
      (bind _output_get_18 (Variables|MIDynamic|SetMaterial%20Footprint%20Ideal _returnvalue_20))
      (if (Variables|LeedsUKData|GetSetCountryName?)
        (Rendering|Material|SetScalarParameterValue _output_get_18 "Radius" (Variables|LeedsUKData|Biophysical|GetMaterial%20Footprint%20Under%20%28scaled%29) :!class /Script/Engine.MaterialInstanceDynamic)
        (else
          (Rendering|Material|SetScalarParameterValue _output_get_18 "Radius" (Variables|PlanetaryBoundaryIndicators|Ideal|GetMaterial%20Footprint) :!class /Script/Engine.MaterialInstanceDynamic))))
    (:then_5
      (bind _returnvalue_21 (Rendering|Material|CreateDynamicMaterialInstance (Variables|PlanetaryBoundaryMeshes|Overshoot|Get1__CO2%20Emissions) 0 "/Game/Leeds/Materials/PlanetaryBoundariesOver/MI_CO2EmissionsOver.MI_CO2EmissionsOver" "None" :!class /Script/Engine.PrimitiveComponent))
      (bind _output_get_19 (Variables|MIDynamic|SetCO2%20Emissions%20Over _returnvalue_21))
      (if (Variables|LeedsUKData|GetSetCountryName?)
        (Rendering|Material|SetScalarParameterValue _output_get_19 "Radius" (Variables|LeedsUKData|Biophysical|GetCO2%20Emissions%20Over%20%28scaled%29) :!class /Script/Engine.MaterialInstanceDynamic)
        (else
          (Rendering|Material|SetScalarParameterValue _output_get_19 "Radius" (Variables|PlanetaryBoundaryIndicators|Overshoot|GetCO2%20Emissions%20Overshoot) :!class /Script/Engine.MaterialInstanceDynamic)))
      (bind _returnvalue_22 (Rendering|Material|CreateDynamicMaterialInstance (Variables|PlanetaryBoundaryMeshes|Overshoot|Get2__Phosphorus) 0 "/Game/Leeds/Materials/PlanetaryBoundariesOver/MI_PhosphorusOver.MI_PhosphorusOver" "None" :!class /Script/Engine.PrimitiveComponent))
      (bind _output_get_20 (Variables|MIDynamic|SetPhosphorus%20Over _returnvalue_22))
      (if (Variables|LeedsUKData|GetSetCountryName?)
        (Rendering|Material|SetScalarParameterValue _output_get_20 "Radius" (Variables|LeedsUKData|Biophysical|GetPhosphorus%20Over%20%28scaled%29) :!class /Script/Engine.MaterialInstanceDynamic)
        (else
          (Rendering|Material|SetScalarParameterValue _output_get_20 "Radius" (Variables|PlanetaryBoundaryIndicators|Overshoot|GetPhosphorus%20Overshoot) :!class /Script/Engine.MaterialInstanceDynamic)))
      (bind _returnvalue_23 (Rendering|Material|CreateDynamicMaterialInstance (Variables|PlanetaryBoundaryMeshes|Overshoot|Get3__Nitrogen) 0 "/Game/Leeds/Materials/PlanetaryBoundariesOver/MI_NitrogenOver.MI_NitrogenOver" "None" :!class /Script/Engine.PrimitiveComponent))
      (bind _output_get_21 (Variables|MIDynamic|SetNitrogen%20Over _returnvalue_23))
      (if (Variables|LeedsUKData|GetSetCountryName?)
        (Rendering|Material|SetScalarParameterValue _output_get_21 "Radius" (Variables|LeedsUKData|Biophysical|GetNitrogen%20Over%20%28scaled%29) :!class /Script/Engine.MaterialInstanceDynamic)
        (else
          (Rendering|Material|SetScalarParameterValue _output_get_21 "Radius" (Variables|PlanetaryBoundaryIndicators|Overshoot|GetNitrogen%20Overshoot) :!class /Script/Engine.MaterialInstanceDynamic)))
      (bind _returnvalue_24 (Rendering|Material|CreateDynamicMaterialInstance (Variables|PlanetaryBoundaryMeshes|Overshoot|Get4__Blue%20Water) 0 "/Game/Leeds/Materials/PlanetaryBoundariesOver/MI_BlueWaterOver.MI_BlueWaterOver" "None" :!class /Script/Engine.PrimitiveComponent))
      (bind _output_get_22 (Variables|MIDynamic|SetBlue%20Water%20Over _returnvalue_24))
      (if (Variables|LeedsUKData|GetSetCountryName?)
        (Rendering|Material|SetScalarParameterValue _output_get_22 "Radius" (Variables|LeedsUKData|Biophysical|GetBlue%20Water%20Over%20%28scaled%29) :!class /Script/Engine.MaterialInstanceDynamic)
        (else
          (Rendering|Material|SetScalarParameterValue _output_get_22 "Radius" (Variables|PlanetaryBoundaryIndicators|Overshoot|GetBlue%20Water%20Overshoot) :!class /Script/Engine.MaterialInstanceDynamic)))
      (bind _returnvalue_25 (Rendering|Material|CreateDynamicMaterialInstance (Variables|PlanetaryBoundaryMeshes|Overshoot|Get5__LandUseChange) 0 "/Game/Leeds/Materials/PlanetaryBoundariesOver/MI_LandUseChangeOver.MI_LandUseChangeOver" "None" :!class /Script/Engine.PrimitiveComponent))
      (bind _output_get_23 (Variables|MIDynamic|SetLand%20Use%20Change%20Over _returnvalue_25))
      (if (Variables|LeedsUKData|GetSetCountryName?)
        (Rendering|Material|SetScalarParameterValue _output_get_23 "Radius" (Variables|LeedsUKData|Biophysical|GetLand%20Use%20Change%20Over%20%28scaled%29) :!class /Script/Engine.MaterialInstanceDynamic)
        (else
          (Rendering|Material|SetScalarParameterValue _output_get_23 "Radius" (Variables|PlanetaryBoundaryIndicators|Overshoot|GetLand%20Use%20Change%20Overshoot) :!class /Script/Engine.MaterialInstanceDynamic)))
      (bind _returnvalue_26 (Rendering|Material|CreateDynamicMaterialInstance (Variables|PlanetaryBoundaryMeshes|Overshoot|Get6__EcologicalFootprint) 0 "/Game/Leeds/Materials/PlanetaryBoundariesOver/MI_EcologicalFootprintOver.MI_EcologicalFootprintOver" "None" :!class /Script/Engine.PrimitiveComponent))
      (bind _output_get_24 (Variables|MIDynamic|SetEcological%20Footprint%20Over _returnvalue_26))
      (if (Variables|LeedsUKData|GetSetCountryName?)
        (Rendering|Material|SetScalarParameterValue _output_get_24 "Radius" (Variables|LeedsUKData|Biophysical|GetEcological%20Footprint%20Over%20%28scaled%29) :!class /Script/Engine.MaterialInstanceDynamic)
        (else
          (Rendering|Material|SetScalarParameterValue _output_get_24 "Radius" (Variables|PlanetaryBoundaryIndicators|Overshoot|GetEcological%20Footprint%20Overshoot) :!class /Script/Engine.MaterialInstanceDynamic)))
      (bind _returnvalue_27 (Rendering|Material|CreateDynamicMaterialInstance (Variables|PlanetaryBoundaryMeshes|Overshoot|Get7_MaterialFootprint) 0 "/Game/Leeds/Materials/PlanetaryBoundariesOver/MI_MaterialFootprintOver.MI_MaterialFootprintOver" "None" :!class /Script/Engine.PrimitiveComponent))
      (bind _output_get_25 (Variables|MIDynamic|SetMaterial%20Footprint%20Over _returnvalue_27))
      (if (Variables|LeedsUKData|GetSetCountryName?)
        (Rendering|Material|SetScalarParameterValue _output_get_25 "Radius" (Variables|LeedsUKData|Biophysical|GetMaterial%20Footprint%20Over%20%28scaled%29) :!class /Script/Engine.MaterialInstanceDynamic)
        (else
          (Rendering|Material|SetScalarParameterValue _output_get_25 "Radius" (Variables|PlanetaryBoundaryIndicators|Overshoot|GetMaterial%20Footprint%20Overshoot) :!class /Script/Engine.MaterialInstanceDynamic))))))

(fn SetMarkerCountryName
  (Development|PrintString "Setting Marker Name")
  (Variables|LeedsUKData|SetSetCountryName? false)
  (bind _output_get (Variables|LeedsUKData|SetCountryName "NewEnumerator9"))
  (Development|PrintString (Utilities|String|EnumtoString _output_get))
  (Variables|LeedsUKData|SetSetCountryName? true))